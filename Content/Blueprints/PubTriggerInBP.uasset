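; Pub entrance trigger that switches the music and teleports the Avatar behind a screen fade.
; On any overlap, it fades out the BP_SPHINXPlayerController's MainAudio and immediately plays a Suikoden II theme, before checking that the overlapping actor is an Avatar.
; For an Avatar, it plays WBP_Fade, moves the actor to NewLocation, reverses the fade and removes the widget, using short delays between steps.
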(event Collision|EventActorBeginOverlap
  (params (OtherActor :type Actor%20Object%20Reference))
  (bind _asbp_sphinxplayer_controller (Utilities|Casting|CastToBP_SPHINXPlayerController (Game|GetPlayerController 0)))
  (Audio|Components|Audio|FadeOut (Variables|/Game/Blueprints/BP_SPHINXPlayerController.BP_SPHINXPlayerController_C|GetMainAudio _asbp_sphinxplayer_controller) 1.0 0.0 "Linear" :!class /Script/Engine.AudioComponent)
  (Audio|Components|Audio|SetSound (Variables|/Game/Blueprints/BP_SPHINXPlayerController.BP_SPHINXPlayerController_C|GetMainAudio _asbp_sphinxplayer_controller) "/Game/Sound/Suikoden_II_-_Heart_Softening_Theme___HQ_theme__1__extended_to_20_minutes_.Suikoden_II_-_Heart_Softening_Theme___HQ_theme__1__extended_to_20_minutes_")
  (Audio|Components|Audio|Play (Variables|/Game/Blueprints/BP_SPHINXPlayerController.BP_SPHINXPlayerController_C|GetMainAudio _asbp_sphinxplayer_controller) 0.0)
  (bind _asavatar (Utilities|Casting|CastToAvatar OtherActor))
  (bind _returnvalue (UserInterface|CreateWidget "/Game/UI/UI_BPs/WBP_Fade.WBP_Fade_C"))
  (bind _output_get (Variables|Default|SetFadeWidget _returnvalue))
  (UserInterface|Viewport|AddtoViewport _output_get 0)
  (UserInterface|Animation|PlayAnimation _output_get (Variables|/Game/UI/UI_BPs/WBP_Fade.WBP_Fade_C|GetFadeAnim _output_get) 0.0 1 "Forward" 1.0 false)
  (Utilities|FlowControl|Delay 0.5)
  (Transformation|SetActorLocation _asavatar (Variables|Default|GetNewLocation) false false)
  (UserInterface|Animation|PlayAnimation (Variables|Default|GetFadeWidget) (Variables|/Game/UI/UI_BPs/WBP_Fade.WBP_Fade_C|GetFadeAnim (Variables|Default|GetFadeWidget)) 0.0 1 "Reverse" 1.0 false)
  (Utilities|FlowControl|Delay 0.5)
  (Widget|RemovefromParent (Variables|Default|GetFadeWidget)))

(fn ConstructionScript)