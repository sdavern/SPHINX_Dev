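; TriggerBP is a trigger actor that moves the Avatar to a set NewLocation behind a screen fade.
; On overlap by an Avatar, it creates a WBP_Fade widget, adds it to the viewport and plays FadeAnim.
; After a short delay it relocates the Avatar without sweep, plays the animation in reverse, then removes the widget after another delay.
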(event Collision|EventActorBeginOverlap
  (params (OtherActor :type Actor%20Object%20Reference))
  (bind _asavatar (Utilities|Casting|CastToAvatar OtherActor))
  (bind _returnvalue (UserInterface|CreateWidget "/Game/UI/UI_BPs/WBP_Fade.WBP_Fade_C"))
  (bind _output_get (Variables|Default|SetFadeWidget _returnvalue))
  (UserInterface|Viewport|AddtoViewport _output_get 0)
  (UserInterface|Animation|PlayAnimation _output_get (Variables|/Game/UI/UI_BPs/WBP_Fade.WBP_Fade_C|GetFadeAnim _output_get) 0.0 1 "Forward" 1.0 false)
  (Utilities|FlowControl|Delay 0.5)
  (Transformation|SetActorLocation _asavatar (Variables|Default|GetNewLocation) false false)
  (UserInterface|Animation|PlayAnimation (Variables|Default|GetFadeWidget) (Variables|/Game/UI/UI_BPs/WBP_Fade.WBP_Fade_C|GetFadeAnim (Variables|Default|GetFadeWidget)) 0.0 1 "Reverse" 1.0 false)
  (Utilities|FlowControl|Delay 0.5)
  (Widget|RemovefromParent (Variables|Default|GetFadeWidget)))

(fn ConstructionScript)