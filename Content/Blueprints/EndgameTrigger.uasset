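; Endgame trigger actor that shows the EndScene widget and disables the player Avatar's input when an actor overlaps it.
; On overlap it fetches BP_PuzzleManager and compares completed puzzles to the maximum, but both branches are empty, so the ending does not depend on that check.
; The overlapping actor is not checked; the Avatar and controller come from player index 0.
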(event EventBeginPlay)

(event Collision|EventActorBeginOverlap
  (params (OtherActor :type Actor%20Object%20Reference))
  (bind _returnvalue (Actor|GetActorOfClass "/Game/BP_PuzzleManager.BP_PuzzleManager_C"))
  (bind _output_get (Variables|Default|SetPMInstance _returnvalue))
  (if (== (Variables|/Script/SPHINX_Dev.PuzzleManager|GetMaxPuzzles _output_get) (Variables|/Script/SPHINX_Dev.PuzzleManager|GetCompletedPuzzles _output_get))
    _
    (else
      _))
  (bind _returnvalue_2 (Game|ConstructObjectfromClass "/Game/UI/UI_BPs/EndScene.EndScene_C"))
  (bind _asavatar (Utilities|Casting|CastToAvatar (Game|Player|GetPlayerPawn 0)))
  (bind _assphinx_dev_player_controller (Utilities|Casting|CastToSPHINX_DevPlayerController (Game|GetPlayerController 0)))
  (Input|DisableInput _asavatar _assphinx_dev_player_controller)
  (UserInterface|Viewport|AddtoViewport _returnvalue_2 1))

(fn ConstructionScript)